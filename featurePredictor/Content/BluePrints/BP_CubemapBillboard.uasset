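; Cubemap billboard actor that shows video frames on six faces: top, bottom, rear, left, front and right.
; On BeginPlay it enables input, applies ViewRatio to the MyPawn camera, then creates a dynamic material instance per billboard, only if the pawn cast succeeds.
; OnNextVideoFrame pushes each face's texture variable into the "Texture" parameter of its material; those textures are not assigned in this graph.
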(event `self.ReceiveBeginPlay`
  ;[1 1 1] 카메라 시야 조절
  (`self.EnableInput` (`GameplayStatics.GetPlayerController` 0))
  (bind _asmy_pawn (cast `MyPawn` (`GameplayStatics.GetPlayerPawn` 0)))
  (`CameraComponent.SetAspectRatio` (`MyPawn.Camera` _asmy_pawn) (`self.ViewRatio`))
  (bind _returnvalue (`PrimitiveComponent.CreateDynamicMaterialInstance` (`self.BillboardTop`) 0 "/Game/Materials/M_Top.M_Top"))
  (set `self.DMTop` _returnvalue)
  (bind _returnvalue_2 (`PrimitiveComponent.CreateDynamicMaterialInstance` (`self.BillboardBottom`) 0 "/Game/Materials/M_Bottom.M_Bottom"))
  (set `self.DMBottom` _returnvalue_2)
  (bind _returnvalue_3 (`PrimitiveComponent.CreateDynamicMaterialInstance` (`self.BillboardRear`) 0 "/Game/Materials/M_Rear.M_Rear"))
  (set `self.DMRear` _returnvalue_3)
  (bind _returnvalue_4 (`PrimitiveComponent.CreateDynamicMaterialInstance` (`self.BillboardLeft`) 0 "/Game/Materials/M_Left.M_Left"))
  (set `self.DMLeft` _returnvalue_4)
  (bind _returnvalue_5 (`PrimitiveComponent.CreateDynamicMaterialInstance` (`self.BillboardFront`) 0 "/Game/Materials/M_Front.M_Front"))
  (set `self.DMFront` _returnvalue_5)
  (bind _returnvalue_6 (`PrimitiveComponent.CreateDynamicMaterialInstance` (`self.BillBoardRight`) 0 "/Game/Materials/M_Right.M_Right"))
  (set `self.DMRight` _returnvalue_6))

(event `self.OnNextVideoFrame`
  (`MaterialInstanceDynamic.SetTextureParameterValue` (`self.DMTop`) "Texture" (`self.TopTexture`))
  (`MaterialInstanceDynamic.SetTextureParameterValue` (`self.DMBottom`) "Texture" (`self.BottomTexture`))
  (`MaterialInstanceDynamic.SetTextureParameterValue` (`self.DMRear`) "Texture" (`self.RearTexture`))
  (`MaterialInstanceDynamic.SetTextureParameterValue` (`self.DMLeft`) "Texture" (`self.LeftTexture`))
  (`MaterialInstanceDynamic.SetTextureParameterValue` (`self.DMFront`) "Texture" (`self.FrontTexture`))
  (`MaterialInstanceDynamic.SetTextureParameterValue` (`self.DMRight`) "Texture" (`self.RightTexture`)))

(fn `UserConstructionScript`)